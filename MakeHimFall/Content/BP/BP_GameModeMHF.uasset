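; Game mode that sets up the match for a tower master and a jumper, switching the default pawn to BP_Jumper on BeginPlay.
; On PostLogin, after a five-second delay, it readies the last BP_TowerMaster found, sets up its camera, shows a Timer widget for player 0 and sets the game instance's TimerGO flag.
; JumperReady similarly readies a BP_Jumper and its camera, then sets TimerGO.
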(event `self.ReceiveBeginPlay`
  ;[0.7197 0 1] Switch default character spawn
  (set `self.DefaultPawnClass` "/Game/BP/Characters/BP_Jumper.BP_Jumper_C"))

(event `self.K2_PostLogin`
  (params (NewPlayer :type "PlayerController Object Reference"))
  (bind _outactors (`GameplayStatics.GetAllActorsOfClass` "/Game/BP/Characters/BP_TowerMaster.BP_TowerMaster_C"))
  (for _array_element _outactors
    _)
  (`KismetSystemLibrary.Delay` 5.0)
  (bind _asbp_tower_master (cast `/Game/BP/Characters/BP_TowerMaster` _array_element))
  (set `/Game/BP/Characters/BP_TowerMaster.ready` true _asbp_tower_master)
  (`/Game/BP/Characters/BP_TowerMaster.SetupCamera` _asbp_tower_master)
  (bind _returnvalue (`|CreateWidget` "/Game/UI/Timer.Timer_C" (`GameplayStatics.GetPlayerController` 0)))
  (`UserWidget.AddToViewport` _returnvalue 0)
  (bind _asbp_game_instance (cast `/Game/BP/BP_GameInstance` (`GameplayStatics.GetGameInstance`)))
  (set `/Game/BP/BP_GameInstance.TimerGO` true _asbp_game_instance))

(event `JumperReady`
  (bind _outactors (`GameplayStatics.GetAllActorsOfClass` "/Game/BP/Characters/BP_Jumper.BP_Jumper_C"))
  (for _array_element _outactors
    _)
  (`KismetSystemLibrary.Delay` 5.0)
  (bind _asbp_jumper (cast `/Game/BP/Characters/BP_Jumper` _array_element))
  (set `/Game/BP/Characters/BP_Jumper.ready` true _asbp_jumper)
  (`/Game/BP/Characters/BP_Jumper.SetupCamera` _asbp_jumper)
  (set `self.TimerGO` true))

(fn `UserConstructionScript`)