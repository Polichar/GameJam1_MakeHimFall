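; BP_TowerMaster is a player-controlled tower master that slides its TowerMaster component along X and Z once Ready, and triggers traps in the multiplayer game.
; ActiveTrap box-traces at that component, matches the hit actor's class against TrapName, then casts by index to set the punch, floor, shooter or slower trap's activation flag.
; It also toggles the multiplayer menu, reveals the component on authority, and offers SetupCamera to reset its height.
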(event `InputAction|MenuMultijoueur`
  (params (Key :type "Key Structure"))
  (bind _returnvalue (`GameplayStatics.GetPlayerController` 0))
  ;[1 1 1] Menu Multiplayer
  (:`Pressed`
    (`/Engine/EditorBlueprintResources/StandardMacros.FlipFlop`
      (:`A`
        (set `PlayerController.bShowMouseCursor` true _returnvalue)
        (bind _returnvalue_2 (`|CreateWidget` "/Game/UI/mainMenu.mainMenu_C" _returnvalue))
        (`UserWidget.AddToViewport` _returnvalue_2 0))
      (:`B`
        (set `PlayerController.bShowMouseCursor` false _returnvalue)
        (`WidgetLayoutLibrary.RemoveAllWidgets`)))))

(event `InputAxis|MoveForward`
  (params (AxisValue :type "Float (single-precision)"))
  ;[1 0 0] Movement
  (if (`self.ready`)
    (`SceneComponent.K2_AddLocalOffset` (`self.towerMaster`) (`KismetMathLibrary.MakeVector` 0.0 0.0 (* AxisValue (`self.SpeedTowerMaster`))) false false)))

(event `InputAxis|MoveRight`
  (params (AxisValue :type "Float (single-precision)"))
  ;[1 0 0] Movement
  (if (`self.ready`)
    (`SceneComponent.K2_AddLocalOffset` (`self.towerMaster`) (`KismetMathLibrary.MakeVector` (* AxisValue (`self.SpeedTowerMaster`))) false false)))

(event `self.ReceiveBeginPlay`
  (`self.K2_AddActorLocalOffset` (0.0 20.0 0.0))
  (`/Engine/EditorBlueprintResources/ActorMacros.Switch Has Authority`
    (:`Authority`
      (`SceneComponent.SetVisibility` (`self.towerMaster`) true false))))

(event `InputAction|ActiveTrap`
  (params (Key :type "Key Structure"))
  (bind (_returnvalue_x _returnvalue_y _returnvalue_z) (`KismetMathLibrary.BreakVector` (`SceneComponent.K2_GetComponentLocation` (`self.towerMaster`))))
  (bind _returnvalue (+ _returnvalue_x -5.0))
  (bind _returnvalue_2 (+ _returnvalue_z 10.0))
  ;[1 0 0.8061] Object detection when click
  (:`Pressed`
    (bind _outhit (`KismetSystemLibrary.BoxTraceSingle` (`KismetMathLibrary.MakeVector` _returnvalue _returnvalue_y _returnvalue_2) (`KismetMathLibrary.MakeVector` _returnvalue _returnvalue_y _returnvalue_2) (5.0 100.0 5.0) (struct) "TraceTypeQuery1"))
    (for (_array_element _array_index) (`self.TrapName`) :!label _label
      (if (== _array_element (`GameplayStatics.GetObjectClass` (`.HitActor` (`GameplayStatics.BreakHitResult` _outhit))))
        (set `self.IndexTrap` _array_index)
        (`self.TrapFound`)))
    (switch `int` (`self.IndexTrap`)
      (:`0`
        (bind _asbp_trap_punch (cast `/Game/BP/Traps/BP_TrapPunch` (`.HitActor` (`GameplayStatics.BreakHitResult` _outhit))))
        (set `/Game/BP/Traps/BP_TrapPunch.TrapPunchActivated` true _asbp_trap_punch))
      (:`1`
        (bind _asbp_trap_floor (cast `/Game/BP/Traps/BP_TrapFloor` (`.HitActor` (`GameplayStatics.BreakHitResult` _outhit))))
        (set `/Game/BP/Traps/BP_TrapFloor.TrapFloorActivated` true _asbp_trap_floor))
      (:`2`
        (bind _asbp_trap_support_shooter (cast `/Game/BP/Traps/BP_TrapSupportShooter` (`.HitActor` (`GameplayStatics.BreakHitResult` _outhit))))
        (set `/Game/BP/Traps/BP_TrapSupportShooter.TrapShooterActivated` true _asbp_trap_support_shooter))
      (:`3`
        (bind _asbp_trap_support_slower (cast `/Game/BP/Traps/BP_TrapSupportSlower` (`.HitActor` (`GameplayStatics.BreakHitResult` _outhit))))
        (set `/Game/BP/Traps/BP_TrapSupportSlower.TrapSlowerActivated` true _asbp_trap_support_slower)))))

(event `TrapFound`
  ;[1 0 0.8061] Object detection when click
  (goto _label :!via `Break`))

(event `SetupCamera`
  (bind _towermaster (`self.towerMaster`))
  (bind (_returnvalue_x _returnvalue_y) (`KismetMathLibrary.BreakVector` (`SceneComponent.K2_GetComponentLocation` _towermaster)))
  (`SceneComponent.K2_SetWorldLocation` _towermaster (`KismetMathLibrary.MakeVector` _returnvalue_x _returnvalue_y -1890.0) false false))

(fn `UserConstructionScript`)