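; BP_Jumper is a side-scrolling player character that moves along world X and jumps.
; While falling, horizontal input also triggers a local X offset by CounterJumpForce, signed against the input as a small counter force.
; A menu input uses a FlipFlop to alternate between showing the cursor with a new MainMenu widget and hiding the cursor while removing all widgets.
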(event `InputAction|MenuMultijoueur`
  (params (Key :type "Key Structure"))
  (bind _returnvalue (`GameplayStatics.GetPlayerController` 0))
  ;[1 1 1] Menu Multiplayer
  (:`Pressed`
    (`/Engine/EditorBlueprintResources/StandardMacros.FlipFlop`
      (:`A`
        (set `PlayerController.bShowMouseCursor` true _returnvalue)
        (bind _returnvalue_2 (`|CreateWidget` "/Game/UI/mainMenu.mainMenu_C" _returnvalue))
        (`UserWidget.AddToViewport` _returnvalue_2 0))
      (:`B`
        (set `PlayerController.bShowMouseCursor` false _returnvalue)
        (`WidgetLayoutLibrary.RemoveAllWidgets`)))))

(event `InputAxis|MoveRight`
  (params (AxisValue :type "Float (single-precision)"))
  (bind _counter_jump_force (`self.Counter jump force`))
  ;[1 0 0] Movement
  (`self.AddMovementInput` (1.0 0.0 0.0) AxisValue)
  ;[1 0 0.75] Small counter force
  (if (and (!= AxisValue 0.0) (`NavMovementComponent.IsFalling` (`self.CharacterMovement`)))
    (`/Engine/EditorBlueprintResources/StandardMacros.CompareFloat` AxisValue
      (:`>`
        (`self.K2_AddActorLocalOffset` (`KismetMathLibrary.MakeVector` (* _counter_jump_force -1.0))))
      (:`<`
        (`self.K2_AddActorLocalOffset` (`KismetMathLibrary.MakeVector` _counter_jump_force))))))

(event `InputAction|Jump`
  (params (Key :type "Key Structure"))
  ;[1 0 0] Movement
  (:`Pressed`
    (`self.Jump`))
  (:`Released`
    (`self.StopJumping`)))

(fn `UserConstructionScript`)