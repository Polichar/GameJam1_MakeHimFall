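; BP_TrapBalleShoot is a parrot projectile trap that knocks the jumper when its sprite overlaps them.
; It starts a wing-flap sound on spawn and stops it before destroying itself.
; Hitting a BP_Jumper applies an unswept local offset along the sprite's forward vector, scaled by ParrotForce, plays a hurt sound and destroys the parrot immediately.
; Overlapping any other class destroys it after a short delay.
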(event `self.ReceiveBeginPlay`
  (bind _returnvalue (`GameplayStatics.SpawnSound2D` "/Game/Assets/Son/Bird_Flap_01.Bird_Flap_01")))

(event `self.perroquetProjectileSprite.OnComponentBeginOverlap`
  (params (OverlappedComponent :type "PrimitiveComponent Object Reference") (OtherActor :type "Actor Object Reference") (OtherComp :type "PrimitiveComponent Object Reference") (OtherBodyIndex :type Integer) (bFromSweep :type Boolean) (SweepResult :type "HitResult Structure (by ref)"))
  ;[1 0 0] Action projectile
  (if (== (`GameplayStatics.GetObjectClass` OtherActor) "/Game/BP/Characters/BP_Jumper.BP_Jumper_C")
    (`self.K2_AddActorLocalOffset` OtherActor (* (`SceneComponent.GetForwardVector` OverlappedComponent) (`self.Parrot Force`)) false false)
    (`GameplayStatics.PlaySound2D` "/Game/Assets/Son/Hurt_01.Hurt_01")
    (`AudioComponent.Stop` (stale `self.ReceiveBeginPlay` _returnvalue))
    (`self.K2_DestroyActor`)
    (else
      ;;[0 0.4144 1] if no jumper on trajectory
      (`KismetSystemLibrary.Delay` 1.5)
      (`AudioComponent.Stop` (stale `self.ReceiveBeginPlay` _returnvalue))
      (`self.K2_DestroyActor`))))

(fn `UserConstructionScript`)