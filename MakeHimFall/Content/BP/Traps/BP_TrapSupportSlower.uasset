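; BP_TrapSupportSlower is a trap that fires a BP_TrapBalleSlow projectile when its TrapSlowerActivated flag is set.
; Tick polls that flag and the CD readiness boolean, then clears the flag and calls Fire, which spawns the projectile at the MiroirShoot sprite.
; The sprite hides during the CDTime cooldown, then reappears, showing a glow sprite on authority and a different one on remotes.
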(event `Set ready sprite`
  (bind _miroirshoot (`self.MiroirShoot`))
  ;[1 0.04273 0] Set ready sprite
  (`/Engine/EditorBlueprintResources/ActorMacros.Switch Has Authority`
    (:`Authority`
      (`PaperSpriteComponent.SetSprite` _miroirshoot "/Game/Assets/Sprites/Traps/Glow_Tenta_Sprite.Glow_Tenta_Sprite"))
    (:`Remote`
      (`PaperSpriteComponent.SetSprite` _miroirshoot "/Game/Assets/Sprites/Traps/Tombe1_Sprite_0.Tombe1_Sprite_0"))))

(event `self.ReceiveTick`
  (params (DeltaSeconds :type "Float (single-precision)"))
  ;[0 1 0.0615] I'm activated ?
  (if (and (`self.TrapSlowerActivated`) (`self.CD`))
    (set `self.TrapSlowerActivated` false)
    (`self.Fire`)
    (`KismetSystemLibrary.PrintString` "FIRE !")))

(event `Fire`
  (bind _miroirshoot (`self.MiroirShoot`))
  ;[1 0.4256 0.4654] Activer le tir
  (set `self.CD` false)
  (`|SpawnActorFromClass` "/Game/BP/Traps/BP_TrapBalleSlow.BP_TrapBalleSlow_C" (`SceneComponent.K2_GetComponentToWorld` (`self.MiroirShoot`)) "Undefined" "OverrideRootScale" null null)
  (`SceneComponent.SetVisibility` _miroirshoot false false)
  (`KismetSystemLibrary.Delay` (`self.CDTime`))
  (`SceneComponent.SetVisibility` _miroirshoot true false)
  (set `self.CD` true)
  (`self.Set ready sprite`))

(fn `UserConstructionScript`)