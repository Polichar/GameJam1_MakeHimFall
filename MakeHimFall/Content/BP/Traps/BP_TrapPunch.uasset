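; BP_TrapPunch is a punching-glove trap that knocks back a BP_Jumper overlapping its box.
; When TrapPunchActivated is set and cooldown is ready, Tick fires the punch, swapping sprite for flipbook and briefly shifting the box along DirectionFist's forward X component.
; Overlap plays a timeline adding the Repoussoir local offset to the jumper each update.
; The ready glow sprite shows only on authority, returning after the CDTime cooldown.
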(event `self.Box.OnComponentBeginOverlap`
  (params (OverlappedComponent :type "PrimitiveComponent Object Reference") (OtherActor :type "Actor Object Reference") (OtherComp :type "PrimitiveComponent Object Reference") (OtherBodyIndex :type Integer) (bFromSweep :type Boolean) (SweepResult :type "HitResult Structure (by ref)"))
  ;[1 1 1] Repoussement vers la gauche du piege
  (if (== (`GameplayStatics.GetObjectClass` OtherActor) "/Game/BP/Characters/BP_Jumper.BP_Jumper_C")
    (`Timeline|Timeline TrapPunch` :!via `PlayFromStart`
      (:`Update`
        (`self.K2_AddActorLocalOffset` OtherActor (`self.Repoussoir`) false false)))))

(event `self.ReceiveBeginPlay`
  ;[1 0.9001 0] Trap initialization
  (`PaperFlipbookComponent.SetLooping` (`self.Gant_Anim`) true)
  (`self.Set ready sprite`))

(event `Set ready sprite`
  (bind _spritepunch (`self.SpritePunch`))
  ;[1 0.04273 0] Set ready sprite
  (`/Engine/EditorBlueprintResources/ActorMacros.Switch Has Authority`
    (:`Authority`
      (`PaperSpriteComponent.SetSprite` _spritepunch "/Game/Assets/Sprites/Traps/Glow_Gant_Sprite.Glow_Gant_Sprite"))
    (:`Remote`
      (`PaperSpriteComponent.SetSprite` _spritepunch "/Game/Assets/Sprites/Traps/G4_Sprite.G4_Sprite"))))

(event `self.ReceiveTick`
  (params (DeltaSeconds :type "Float (single-precision)"))
  ;[0 1 0.0615] I'm activated ?
  (if (and (`self.TrapPunchActivated`) (`self.CD`))
    (set `self.TrapPunchActivated` false)
    (`self.MakeHimFall`)))

(event `MakeHimFall`
  (bind _gant_anim (`self.Gant_Anim`))
  (bind _box (`self.Box`))
  (bind _spritepunch (`self.SpritePunch`))
  (bind _returnvalue (`SceneComponent.K2_GetComponentLocation` _box))
  (bind _returnvalue_2 (* (`SceneComponent.GetForwardVector` (`self.directionFist`)) (30.0 0.0 0.0)))
  ;[0 1 0.9869] Trap effect launched
  (set `self.CD` false)
  (`SceneComponent.SetVisibility` (`self.SpritePunch`) false false)
  (`SceneComponent.SetVisibility` _gant_anim true false)
  (`PaperFlipbookComponent.PlayFromStart` _gant_anim)
  (`SceneComponent.K2_SetWorldLocation` _box (+ _returnvalue _returnvalue_2) false false)
  (`KismetSystemLibrary.Delay` 0.5)
  (`PaperSpriteComponent.SetSprite` _spritepunch "/Game/Assets/Sprites/Traps/G4_Sprite.G4_Sprite")
  (`SceneComponent.SetVisibility` _spritepunch true false)
  (`SceneComponent.SetVisibility` (`self.Gant_Anim`) false false)
  (`SceneComponent.K2_SetWorldLocation` _box (+ _returnvalue (* _returnvalue_2 (-1.0 0.0 0.0))) false false)
  (`KismetSystemLibrary.Delay` (`self.CDTime`))
  (set `self.CD` true)
  (`self.Set ready sprite`))

(fn `UserConstructionScript`)