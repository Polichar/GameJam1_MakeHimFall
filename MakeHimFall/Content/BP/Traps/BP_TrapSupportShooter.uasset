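; BP_TrapSupportShooter is a shooter trap that fires a BP_TrapBalleShoot projectile when activated.
; Tick polls the TrapShooterActivated flag and, if the cooldown flag CD is set, spawns the projectile at DirectionCanard's transform.
; Firing hides the MiroirShoot sprite for CDTime, then restores it.
; The ready sprite uses SwitchHasAuthority, showing a glowing parrot on authority and a different parrot sprite on remotes.
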(event `self.ReceiveBeginPlay`
  ;[1 0.5331 0.9326] Start Sprite
  (`self.Set ready sprite`))

(event `self.ReceiveTick`
  (params (DeltaSeconds :type "Float (single-precision)"))
  ;[0 1 0.0615] I'm activated ?
  (if (and (`self.TrapShooterActivated`) (`self.CD`))
    (set `self.TrapShooterActivated` false)
    (`self.Fire`)))

(event `Set ready sprite`
  (bind _miroirshoot (`self.MiroirShoot`))
  ;[1 0.04273 0] Set ready sprite
  (`/Engine/EditorBlueprintResources/ActorMacros.Switch Has Authority`
    (:`Authority`
      (`PaperSpriteComponent.SetSprite` _miroirshoot "/Game/Assets/Sprites/Traps/Glow_Perroquet_Sprite.Glow_Perroquet_Sprite"))
    (:`Remote`
      (`PaperSpriteComponent.SetSprite` _miroirshoot "/Game/Assets/Sprites/Traps/Perroquet1_Sprite_0.Perroquet1_Sprite_0"))))

(event `Fire`
  (bind _miroirshoot (`self.MiroirShoot`))
  ;[1 0.4256 0.4654] Activer le tir
  (set `self.CD` false)
  (`|SpawnActorFromClass` "/Game/BP/Traps/BP_TrapBalleShoot.BP_TrapBalleShoot_C" (`SceneComponent.K2_GetComponentToWorld` (`self.DirectionCanard`)) "Undefined" "OverrideRootScale" null null)
  (`SceneComponent.SetVisibility` _miroirshoot false false)
  (`KismetSystemLibrary.Delay` (`self.CDTime`))
  (set `self.CD` true)
  (`SceneComponent.SetVisibility` _miroirshoot true false)
  (`self.Set ready sprite`))

(fn `UserConstructionScript`)