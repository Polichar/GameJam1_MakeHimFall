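; BP_TrapFloor is a trap floor platform, built on a sprite, that drops away when activated and later restores itself.
; Tick polls TrapFloorActivated, clears it and runs MakeHimFall, which shows the destroyed sprite, waits, then hides the plate and sets collision to overlap.
; After a cooldown it restores visibility and blocking collision.
; The ready sprite depends on authority: glowing on authority, destroyed-platform art on remote.
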(event `Set ready sprite`
  (bind _plaquetrappe (`self.PlaqueTrappe`))
  ;[1 0.04273 0] Set ready sprite
  (`/Engine/EditorBlueprintResources/ActorMacros.Switch Has Authority`
    (:`Authority`
      (`PaperSpriteComponent.SetSprite` _plaquetrappe "/Game/Assets/Sprites/Traps/Glow_Plat_Sprite.Glow_Plat_Sprite"))
    (:`Remote`
      (`PaperSpriteComponent.SetSprite` _plaquetrappe "/Game/Assets/Sprites/Traps/Plateforme_destroy_Sprite.Plateforme_destroy_Sprite"))))

(event `self.ReceiveBeginPlay`
  ;[1 0.5331 0.9326] Start Sprite
  (`self.Set ready sprite`))

(event `MakeHimFall`
  (bind _plaquetrappe (`self.PlaqueTrappe`))
  (bind _plaquetrappe_2 (`self.PlaqueTrappe`))
  ;[0.4766 1 0.9502] Activation du piege
  (`PaperSpriteComponent.SetSprite` _plaquetrappe "/Game/Assets/Sprites/Traps/Plateforme_destroy_Sprite.Plateforme_destroy_Sprite")
  (`KismetSystemLibrary.Delay` (`self.TimeDuration`))
  (`PrimitiveComponent.SetCollisionResponseToAllChannels` _plaquetrappe "ECR_Overlap")
  (`SceneComponent.SetVisibility` _plaquetrappe_2 false false)
  (`KismetSystemLibrary.Delay` (`self.CDTime`))
  (`self.Set ready sprite`)
  (`SceneComponent.SetVisibility` _plaquetrappe_2 true false)
  (`PrimitiveComponent.SetCollisionResponseToAllChannels` _plaquetrappe "ECR_Block"))

(event `self.ReceiveTick`
  (params (DeltaSeconds :type "Float (single-precision)"))
  ;[0 1 0.0615] I'm activated ?
  (if (`self.TrapFloorActivated`)
    (set `self.TrapFloorActivated` false)
    (`self.MakeHimFall`)))

(fn `UserConstructionScript`)